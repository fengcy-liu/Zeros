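; Enemy2 is an enemy character that seeds its Blackboard with a target waypoint actor and dies when its health runs out.
; Damage updates a health bar widget that stays hidden until the first hit.
; Capsule overlaps with an ATCharacter set or clear the IsBlocking Blackboard key.
; Callable events spawn an Enemy_Bomb at a given location and stack walk-speed boosts on the base speed.
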(event `self.ReceiveBeginPlay`
  (bind _targetwaypointactor (`self.TargetWayPointActor`))
  (set `self.Health` (`self.MaxHealth`))
  (`Widget.SetVisibility` (`WidgetComponent.GetUserWidgetObject` (`self.HP_Widget`)) "Hidden")
  (bind _output_get (set `self.BlackBoard` (`AIBlueprintHelperLibrary.GetBlackboard` null)))
  (`BlackboardComponent.SetValueAsObject` _output_get (`KismetSystemLibrary.MakeLiteralName` (`self.BBTargetActorKeyName`)) _targetwaypointactor)
  (set `self.LastWayPointActor` _targetwaypointactor)
  (set `CharacterMovementComponent.MaxWalkSpeed` (`self.BaseMaxWalkSpeed`) (`self.CharacterMovement`)))

(event `self.ReceiveAnyDamage`
  (params (Damage :type "Float (single-precision)") (DamageType :type "DamageType Object Reference") (InstigatedBy :type "Controller Object Reference") (DamageCauser :type "Actor Object Reference"))
  (bind _output_get (set `self.Health` (`KismetMathLibrary.FClamp` (- (`self.Health`) Damage) 0.0 (`self.MaxHealth`))))
  (`self.ShowHealthBar`)
  (if (<= _output_get 0.0)
    (`KismetSystemLibrary.Delay` 0.1)
    (`self.K2_DestroyActor`)))

(event `ShowHealthBar`
  (bind _asumg_enemy_hp (cast `/Game/UI/UMG_EnemyHp` (`WidgetComponent.GetUserWidgetObject` (`self.HP_Widget`))))
  (`/Game/UI/UMG_EnemyHp.SetProgress` _asumg_enemy_hp (/ (`self.Health`) (`self.MaxHealth`)))
  (`/Engine/EditorBlueprintResources/StandardMacros.DoOnce` false
    (:`Completed`
      (`Widget.SetVisibility` _asumg_enemy_hp "Visible"))))

(event `self.Capsule.OnComponentBeginOverlap`
  (params (OverlappedComponent :type "PrimitiveComponent Object Reference") (OtherActor :type "Actor Object Reference") (OtherComp :type "PrimitiveComponent Object Reference") (OtherBodyIndex :type Integer) (bFromSweep :type Boolean) (SweepResult :type "HitResult Structure (by ref)"))
  (cast `/Game/Blueprint/Character/ATCharacter` OtherActor)
  (`BlackboardComponent.SetValueAsBool` (`self.BlackBoard`) "IsBlocking" true))

(event `self.Capsule.OnComponentEndOverlap`
  (params (OverlappedComponent :type "PrimitiveComponent Object Reference") (OtherActor :type "Actor Object Reference") (OtherComp :type "PrimitiveComponent Object Reference") (OtherBodyIndex :type Integer))
  (cast `/Game/Blueprint/Character/ATCharacter` OtherActor)
  (`BlackboardComponent.ClearValue` (`self.BlackBoard`) "IsBlocking"))

(event `SpawnBomb`
  (params (Location :type "Vector Structure"))
  (`|SpawnActorFromClass` "/Game/Blueprint/Enemy/Enemy_Bomb.Enemy_Bomb_C" (`KismetMathLibrary.MakeTransform` Location) "Undefined" "OverrideRootScale" null null))

(event `Acc`
  (bind _output_get (set `self.WalkSpeedCoeff` (+ (`self.WalkSpeedCoeff`) 0.5)))
  (set `CharacterMovementComponent.MaxWalkSpeed` (* _output_get (`self.BaseMaxWalkSpeed`)) (`self.CharacterMovement`)))

(fn `UserConstructionScript`)