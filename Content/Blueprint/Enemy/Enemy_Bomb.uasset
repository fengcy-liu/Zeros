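; Rolling bomb enemy that chases the player and explodes on overlap, dealing damage and destroying itself.
; After a spawn delay it starts an attached sound and, each Tick, eases toward the player in XY until close.
; The sphere yaws toward the player, with roll derived from distance traveled over its radius to fake rolling.
; Damage lowers health, updates a health bar revealed on first hit, and destroys the actor at zero.
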(event `self.ReceiveBeginPlay`
  (set `self.Health` (`self.MaxHealth`))
  (`Widget.SetVisibility` (`WidgetComponent.GetUserWidgetObject` (`self.HP_Widget`)) "Hidden")
  (set `self.lastLocation` (`self.K2_GetActorLocation`))
  (`KismetSystemLibrary.Delay` 5.0)
  (set `self.CanMove` true)
  (`GameplayStatics.SpawnSoundAttached` null (`self.Sphere`) "None" (0.0 0.0 0.0) (struct) "KeepRelativeOffset" true 1.0 1.0 0.0 null null false))

(event `self.ReceiveAnyDamage`
  (params (Damage :type "Float (single-precision)") (DamageType :type "DamageType Object Reference") (InstigatedBy :type "Controller Object Reference") (DamageCauser :type "Actor Object Reference"))
  ;[1 1 1] 受到伤害
  (bind _output_get (set `self.Health` (`KismetMathLibrary.FClamp` (- (`self.Health`) Damage) 0.0 (`self.MaxHealth`))))
  (`self.ShowHealthBar`)
  (if (<= _output_get 0.0)
    (`self.K2_DestroyActor`)))

(event `ShowHealthBar`
  ;[1 1 1] 显示血条
  (bind _asumg_enemy_hp (cast `/Game/UI/UMG_EnemyHp` (`WidgetComponent.GetUserWidgetObject` (`self.HP_Widget`))))
  (`/Game/UI/UMG_EnemyHp.SetProgress` _asumg_enemy_hp (/ (`self.Health`) (`self.MaxHealth`)))
  (`/Engine/EditorBlueprintResources/StandardMacros.DoOnce` false
    (:`Completed`
      (`Widget.SetVisibility` _asumg_enemy_hp "Visible"))))

(event `SphereMove`
  (bind _returnvalue (`self.K2_GetActorLocation`))
  (bind _sphere (`self.Sphere`))
  (bind _returnvalue_roll (`KismetMathLibrary.BreakRotator` (`SceneComponent.K2_GetComponentRotation` _sphere)))
  (bind (_returnvalue_x _returnvalue_y) (`KismetMathLibrary.BreakVector` (`KismetMathLibrary.VInterpTo` _returnvalue (`self.playerLocation`) (`GameplayStatics.GetWorldDeltaSeconds`) 1.0)))
  (bind (_returnvalue_roll_2 _returnvalue_pitch _returnvalue_yaw) (`KismetMathLibrary.BreakRotator` (`KismetMathLibrary.Conv_VectorToRotator` (- (`self.playerLocation`) (`self.K2_GetActorLocation`)))))
  ;[1 1 1] 球体移动和朝向
  (`SceneComponent.K2_SetRelativeRotation` _sphere (`KismetMathLibrary.MakeRotator` _returnvalue_roll 0.0 (+ _returnvalue_yaw 90.0)) false false)
  (`self.K2_SetActorLocation` (`KismetMathLibrary.MakeVector` _returnvalue_x _returnvalue_y (.z _returnvalue))))

(event `SphereRotate`
  ;[1 1 1] 球体移动的旋转变化
  (`SceneComponent.K2_AddRelativeRotation` (`self.Sphere`) (`KismetMathLibrary.MakeRotator` (* (`KismetMathLibrary.RadiansToDegrees` (/ (`KismetMathLibrary.VSize` (- (`self.K2_GetActorLocation`) (`self.lastLocation`))) (`SphereComponent.GetScaledSphereRadius` (`self.Sphere1`)))) -1.0)) false false)
  (set `self.lastLocation` (`self.K2_GetActorLocation`)))

(event `self.ReceiveTick`
  (params (DeltaSeconds :type "Float (single-precision)"))
  (`|ExecutionSequence`
    (:`then_0`
      ;[1 1 1] 判断是否移动
      (if (`self.CanMove`)
        (bind _output_get (set `self.playerLocation` (`self.K2_GetActorLocation` (`GameplayStatics.GetPlayerPawn` 0))))
        (if (>= (`KismetMathLibrary.VSizeXY` (- _output_get (`self.K2_GetActorLocation`))) 70.0)
          (`|ExecutionSequence`
            (:`then_0`
              (`self.SphereRotate`))
            (:`then_1`
              (`self.SphereMove`))))))
    (:`then_1`
      (set `self.SoundInterTime` (+ (`self.SoundInterTime`) DeltaSeconds)))))

(event `self.Sphere2.OnComponentBeginOverlap`
  (params (OverlappedComponent :type "PrimitiveComponent Object Reference") (OtherActor :type "Actor Object Reference") (OtherComp :type "PrimitiveComponent Object Reference") (OtherBodyIndex :type Integer) (bFromSweep :type Boolean) (SweepResult :type "HitResult Structure (by ref)"))
  ;[1 1 1] 碰到玩家爆炸
  (if (`KismetSystemLibrary.DoesImplementInterface` OtherActor "/Game/Blueprint/Character/I_Player.I_Player_C")
    (`GameplayStatics.PlaySoundAtLocation` (`self.Sound`) (`self.K2_GetActorLocation` (`GameplayStatics.GetPlayerPawn` 0)) (struct) 1.0 1.0 0.0 null null null)
    (`GameplayStatics.ApplyDamage` OtherActor 30.0)
    (`self.K2_DestroyActor`)))

(fn `UserConstructionScript`)