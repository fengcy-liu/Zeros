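; Spawner actor that creates successive Enemy2 instances at random WayPoint actors gathered on BeginPlay.
; CreateNewEnemy waits through a delay, then spawns an enemy targeting that waypoint's NextWayPoint, with health and clamped scale growing with SpawnCount.
; It binds an event to each enemy's OnDestroyed, matching CreateNewEnemy's signature to chain respawns until the count limit.
; Nothing in this graph triggers the first spawn.
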(event `self.ReceiveBeginPlay`
  (bind _outactors (`GameplayStatics.GetAllActorsOfClass` "/Game/Blueprint/Enemy/WayPoint.WayPoint_C"))
  (set `self.WayPoint` _outactors))

(event `CreateNewEnemy` :!signature `self.OnDestroyed`
  (params (DestroyedActor :type "Actor Object Reference"))
  (if (<= (`self.spawnCount`) 10)
    (bind _output_get (set `self.CurWayPoint` (`KismetArrayLibrary.Array_Random` (`self.WayPoint`))))
    (`/Engine/EditorBlueprintResources/StandardMacros.IncrementInt` (`self.spawnCount`)
      (:`  `
        (`KismetSystemLibrary.Delay` 5.0)
        (bind _returnvalue (`|SpawnActorFromClass` "/Game/Blueprint/Enemy/Enemy2.Enemy2_C" (`KismetMathLibrary.MakeTransform` (`self.K2_GetActorLocation` (`self.CurWayPoint`)) (struct) (* (0.5 0.5 0.5) (`KismetMathLibrary.Clamp` (`self.spawnCount`) 1 8))) "Undefined" "OverrideRootScale" null (* (`self.spawnCount`) 50.0) (`/Game/Blueprint/Enemy/WayPoint.NextWayPoint` _output_get) null))
        (bind _output_get_2 (set `self.Enemy` _returnvalue))
        (add `self.OnDestroyed` _output_get_2 (`|CreateDelegate` :!event `CreateNewEnemy`))))))

(event `self.ReceiveTick`
  (params (DeltaSeconds :type "Float (single-precision)")))

(fn `UserConstructionScript`)