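; NumActor is a 3D seven-segment digit built from seven static meshes that displays a single number from 0 to 9.
; CreateNum switches to a per-digit function that toggles segment visibility, hiding the whole actor for zero unless CanShowZero is set.
; SetTxture applies one material to every segment.
; When ForcePlayer is on, Tick sets the actor's yaw to face the player pawn, with a fixed offset.
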(event `self.ReceiveBeginPlay`
  (set `self.Pawn` (`GameplayStatics.GetPlayerPawn` 0)))

(event `self.ReceiveTick`
  (params (DeltaSeconds :type "Float (single-precision)"))
  (bind (_returnvalue_roll _returnvalue_pitch _returnvalue_yaw) (`KismetMathLibrary.BreakRotator` (`KismetMathLibrary.FindLookAtRotation` (`self.K2_GetActorLocation`) (`self.K2_GetActorLocation` (`self.Pawn`)))))
  (if (`self.forcePlayer`)
    (`self.K2_SetActorRotation` (`KismetMathLibrary.MakeRotator` 0.0 0.0 (+ _returnvalue_yaw 270.0)))))

(event `CreateNum`
  (params (Num :type Integer))
  (switch `int` Num
    (:`0`
      (if (`self.CanShowZero`)
        (`self.Zero`)
        (else
          (`self.SetActorHiddenInGame` true))))
    (:`1`
      (`self.One`))
    (:`2`
      (`self.Two`))
    (:`3`
      (`self.Three`))
    (:`4`
      (`self.Four`))
    (:`5`
      (`self.Five`))
    (:`6`
      (`self.Six`))
    (:`7`
      (`self.Seven`))
    (:`8`
      (`self.Eight`))
    (:`9`
      (`self.Nine`))))

(event `SetTxture`
  (params (Material :type "MaterialInterface Object Reference"))
  (`PrimitiveComponent.SetMaterial` (`self.StaticMesh2`) 0 Material)
  (`PrimitiveComponent.SetMaterial` (`self.StaticMesh3`) 0 Material)
  (`PrimitiveComponent.SetMaterial` (`self.StaticMesh4`) 0 Material)
  (`PrimitiveComponent.SetMaterial` (`self.StaticMesh5`) 0 Material)
  (`PrimitiveComponent.SetMaterial` (`self.StaticMesh6`) 0 Material)
  (`PrimitiveComponent.SetMaterial` (`self.StaticMesh7`) 0 Material)
  (`PrimitiveComponent.SetMaterial` (`self.StaticMesh1`) 0 Material))

(fn `UserConstructionScript`)