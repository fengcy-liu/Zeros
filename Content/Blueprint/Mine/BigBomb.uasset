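; BigBomb is a self-triggering explosion actor that damages nearby pawns.
; On BeginPlay it waits briefly, then plays an explosion sound and particle effect at its location.
; It damages every pawn overlapping its Sphere once, then destroys itself after a further delay.
; Actor scale drives both the effect's size and the damage, so larger instances hit harder.
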(event `self.ReceiveBeginPlay`
  (bind _returnvalue_x (`KismetMathLibrary.BreakVector` (`self.GetActorScale3D`)))
  (bind _returnvalue (`self.K2_GetActorLocation`))
  (`KismetSystemLibrary.Delay` 0.3)
  (`GameplayStatics.PlaySoundAtLocation` "/Game/Sound/Exp/Wav/SFX_Explosion_01_C.SFX_Explosion_01_C" _returnvalue (struct) 1.0 1.0 0.0 null null null)
  (`GameplayStatics.SpawnEmitterAtLocation` "/Game/M5_Vol1/Particles/Big_Explosion/RealExp_00_A.RealExp_00_A" _returnvalue (struct) (* (`self.GetActorScale3D`) (`self.Scale`)))
  (for _array_element (`PrimitiveComponent.GetOverlappingActors` (`self.Sphere`) "/Script/Engine.Pawn")
    (`GameplayStatics.ApplyDamage` _array_element (* _returnvalue_x (`self.baseDamage`))))
  (`KismetSystemLibrary.Delay` 1.0)
  (`self.K2_DestroyActor`))

(fn `UserConstructionScript`)