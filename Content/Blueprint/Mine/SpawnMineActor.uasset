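; Minefield actor that spawns a Minesweeper-style grid of tiles and tracks safe tiles left and mines triggered.
; SpawnMineTile sizes the box, places mines by swap-based sampling without repeats, spawns the tiles and computes neighbour counts.
; Tile collision events differ by mine status.
; MineCrash spawns or rescales a tracking LockRingActor by crash count, while UpdateResetNum counts down and signals when none remain.
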(event `self.ReceiveBeginPlay`
  (bind _asatgame_mode (cast `/Game/Blueprint/Game/ATGameMode` (`GameplayStatics.GetGameMode`)))
  (set `self.GameMode` _asatgame_mode))

(event `SpawnMineTile`
  (bind (_minesize_x _minesize_y) (`KismetMathLibrary.BreakVector` (`self.MineSize`)))
  (bind (_minesize_x_2 _minesize_y_2 _minesize_z) (`KismetMathLibrary.BreakVector` (`self.MineSize`)))
  ;[1 1 1] 雷区生成
  (set `self.ResetNum` (- (`self.GetMapTileSize`) (`self.MineNum`)))
  (`|ExecutionSequence`
    (:`then_0`
      (`self.SetActorScale3D` (1.0 1.0 1.0))
      (bind _output_get (set `self.BoxRange` (`KismetMathLibrary.MakeVector` (/ (* (`self.Row`) _minesize_x_2) 2.0) (/ (* (`self.Col`) _minesize_y_2) 2.0) _minesize_z)))
      (`BoxComponent.SetBoxExtent` (`self.Box`) _output_get true))
    (:`then_1`
      (`self.RandMineMap` (`self.GetMapTileSize`)))
    (:`then_2`
      (`KismetArrayLibrary.Array_Clear` (`self.MineArr`))
      (for _index (range (`self.GetMapTileSize`))
        (bind _returnvalue (`|SpawnActorFromClass` "/Game/Blueprint/Mine/MineTile.MineTile_C" (`KismetMathLibrary.MakeTransform` (+ (`KismetMathLibrary.MakeVector` (* (`self.GetColIndex` _index) _minesize_y) (* (`self.getRowIndex` _index) _minesize_x)) (/ (`self.MineSize`) 2) (- (`self.K2_GetActorLocation`) (`self.BoxRange`)))) "Undefined" "OverrideRootScale" null (`|GetArrayItem` (`self.IsMine`) _index) false null))
        (`KismetArrayLibrary.Array_Add` (`self.MineArr`) _returnvalue)
        (if (`/Game/Blueprint/Mine/MineTile.IsMine` _returnvalue)
          (add `/Game/Blueprint/Mine/MineTile.CollisionEvent` _returnvalue (`|CreateDelegate` :!event `MineCrash`))
          (else
            (add `/Game/Blueprint/Mine/MineTile.CollisionEvent` _returnvalue (`|CreateDelegate` :!event `UpdateResetNum`))))))
    (:`then_3`
      (for _array_element (`self.MineArr`)
        (`/Game/Blueprint/Mine/MineTile.CalcSuroundMineNum` _array_element)))))

(event `MineCrash`
  ;[1 1 1] 触碰陷阱的事件
  (`/Engine/EditorBlueprintResources/StandardMacros.IncrementInt` (`self.CrashMineCount`)
    (:`  `
      (bind _returnvalue (`GameplayStatics.GetActorOfClass` "/Game/Blueprint/Mine/LockRingActor.LockRingActor_C"))
      (`/Engine/EditorBlueprintResources/StandardMacros.IsValid` _returnvalue
        (:`Is Valid`
          (`self.SetActorScale3D` _returnvalue (* (`self.BaseRingScale`) (`self.CrashMineCount`))))
        (:`Is Not Valid`
          (bind _returnvalue_2 (`|SpawnActorFromClass` "/Game/Blueprint/Mine/LockRingActor.LockRingActor_C" (`KismetMathLibrary.MakeTransform` (`self.K2_GetActorLocation`) (struct) (* (`self.BaseRingScale`) (`KismetMathLibrary.Max` (- (`self.CrashMineCount`) 1) 1))) "Undefined" "OverrideRootScale" null null))
          (`/Game/Blueprint/Mine/LockRingActor.SetTracking` _returnvalue_2))))))

(event `UpdateResetNum`
  (bind _resetnum (`self.ResetNum`))
  (bind _result (`/Engine/EditorBlueprintResources/StandardMacros.DecrementInt` _resetnum)
    (:`  `
      (`self.NumChanged` _resetnum)
      (if (<= _result 0)
        (`self.NumBeZeros`)))))

(fn `GetColIndex`
  (params (Index :type Integer))
  (returns (val :type Integer))
  (return (mod Index (`self.Col`))))

(fn `GetMapTileSize`
  (returns (TileNum :type Integer))
  (return (* (`self.Row`) (`self.Col`))))

(fn `GetRowIndex`
  (params (Index :type Integer))
  (returns (val :type Integer))
  (return (/ Index (`self.Col`))))

(fn `RandMineMap`
  (params (Size :type Integer))
  (locals (IndexArr :type "Array of Integer") (LastIndex :type Integer) (RandIndex :type Integer :default 0))
  (bind _lastindex (`local.LastIndex`))
  (set `local.LastIndex` (- Size 1))
  (`KismetArrayLibrary.Array_Resize` (`local.IndexArr`) Size)
  (`KismetArrayLibrary.Array_Resize` (`self.IsMine`) Size)
  (for _index (range Size)
    (`KismetArrayLibrary.Array_Set` (`local.IndexArr`) _index _index)
    (`KismetArrayLibrary.Array_Set` (`self.IsMine`) _index))
  (`|ExecutionSequence`
    (:`then_0`
      (for _ (range 1 (+ (`self.MineNum`) 1))
        (bind _output_get (set `local.RandIndex` (`KismetMathLibrary.RandomInteger` (+ (`local.LastIndex`) 1))))
        (`KismetArrayLibrary.Array_Set` (`self.IsMine`) (`|GetArrayItem` (`local.IndexArr`) _output_get) true)
        (`KismetArrayLibrary.Array_Swap` (`local.IndexArr`) _output_get _lastindex)
        (`/Engine/EditorBlueprintResources/StandardMacros.DecrementInt` _lastindex))
      (return))))

(fn `UserConstructionScript`)