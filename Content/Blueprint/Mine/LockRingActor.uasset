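; Targeting ring actor that chases the player and drops a BigBomb where it locks on.
; Tracking starts shortly after BeginPlay, easing toward the player pawn in XY using accumulated, clamped time as the interpolation delta.
; Staying inside a radius derived from decal size for MinLockedDuration fires a DoOnce lock, which spawns the bomb after a brief delay and destroys the ring.
; Decal materials signal each state; RemoveTracking hides the ring.
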(event `Locked`
  (params (Location :type "Vector Structure"))
  (`KismetSystemLibrary.Delay` 0.2)
  (`DecalComponent.SetDecalMaterial` (`self.Decal`) (`self.Locked Decal Material`))
  (`|SpawnActorFromClass` "/Game/Blueprint/Mine/BigBomb.BigBomb_C" (`KismetMathLibrary.MakeTransform` Location (struct) (`self.GetActorScale3D`)) "Undefined" "OverrideRootScale" null null)
  (set `self.IsTracking` false)
  (`self.K2_DestroyActor`))

(event `SetTracking`
  (set `self.IsTracking` true)
  (`self.SetActorHiddenInGame` false)
  (set `self.DurationTime` 0.0)
  (set `self.deltaSecond` 0.0)
  (`DecalComponent.SetDecalMaterial` (`self.Decal`) (`self.Unlocked Decal Material`))
  (goto _label :!via `Reset`))

(event `self.ReceiveBeginPlay`
  (`KismetSystemLibrary.Delay` 2.0)
  (`self.SetTracking`))

(event `RemoveTracking`
  (set `self.IsTracking` false)
  (`self.SetActorHiddenInGame` true))

(event `self.ReceiveTick`
  (params (DeltaSeconds :type "Float (single-precision)"))
  (bind (_returnvalue_x _returnvalue_y _returnvalue_z) (`KismetMathLibrary.BreakVector` (`self.K2_GetActorLocation`)))
  (bind (_returnvalue_x_2 _returnvalue_y_2) (`KismetMathLibrary.BreakVector` (`self.GetActorScale3D`)))
  (bind (_decalsize_x _decalsize_y) (`KismetMathLibrary.BreakVector` (`DecalComponent.DecalSize` (`self.Decal`))))
  (if (`self.IsTracking`)
    (bind _output_get (set `self.deltaSecond` (+ (`self.deltaSecond`) DeltaSeconds)))
    (`self.K2_SetActorLocation` (`KismetMathLibrary.MakeVector` (.x (`KismetMathLibrary.VInterpTo` (`self.K2_GetActorLocation`) (`self.K2_GetActorLocation` (`GameplayStatics.GetPlayerPawn` 0)) (`KismetMathLibrary.FClamp` _output_get 0.0 0.5) 0.2)) (.y (`KismetMathLibrary.VInterpTo` (`self.K2_GetActorLocation`) (`self.K2_GetActorLocation` (`GameplayStatics.GetPlayerPawn` 0)) (`KismetMathLibrary.FClamp` _output_get 0.0 0.5) 0.2)) _returnvalue_z))
    (if (< (`KismetMathLibrary.Vector_Distance2D` (`self.K2_GetActorLocation`) (`self.K2_GetActorLocation` (`GameplayStatics.GetPlayerPawn` 0))) (/ (* _decalsize_y _returnvalue_y_2) 4.0))
      (bind _output_get_2 (set `self.DurationTime` (+ (`self.DurationTime`) (`GameplayStatics.GetWorldDeltaSeconds`))))
      (if (> _output_get_2 (`self.MinLockedDuration`))
        (`/Engine/EditorBlueprintResources/StandardMacros.DoOnce` true :!label _label
          (:`Completed`
            (`DecalComponent.SetDecalMaterial` (`self.Decal`) (`self.Locking Decal Material`))
            (`self.Locked` (`self.K2_GetActorLocation`)))))
      (else
        (set `self.DurationTime` 0.0)))))

(fn `UserConstructionScript`)