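; DoorCount is a two-panel sliding door with a two-digit number display.
; UpdateNum reveals the hidden NumActor child actors on first use, then feeds them the ones and tens digits of the value clamped to 0–99.
; OpenDoor and CloseDoor play or reverse the Open timeline, sliding both meshes along X in proportion to their starting offsets.
; A Character entering the box triggers the LeaveDoor call.
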(event `self.ReceiveBeginPlay`
  (set `self.StaticMesh1Location` (`SceneComponent.RelativeLocation` (`self.StaticMesh1`)))
  (set `self.StaticMesh2Location` (`SceneComponent.RelativeLocation` (`self.StaticMesh2`)))
  (`SceneComponent.SetVisibility` (`self.ChildActor1`) false false)
  (`SceneComponent.SetVisibility` (`self.ChildActor2`) false false))

(event `UpdateNum`
  (params (Num :type Integer))
  (bind _returnvalue (`KismetMathLibrary.Clamp` Num 0 99))
  (bind _asnum_actor (cast `/Game/Blueprint/Mine/NumActor` (`ChildActorComponent.ChildActor` (`self.ChildActor2`)) :!pure true))
  (bind _asnum_actor_2 (cast `/Game/Blueprint/Mine/NumActor` (`ChildActorComponent.ChildActor` (`self.ChildActor1`)) :!pure true))
  (`|ExecutionSequence`
    (:`then_0`
      (`/Engine/EditorBlueprintResources/StandardMacros.DoOnce` false
        (:`Completed`
          (`SceneComponent.SetVisibility` (`self.ChildActor1`) true false)
          (`SceneComponent.SetVisibility` (`self.ChildActor2`) true false)
          (set `/Game/Blueprint/Mine/NumActor.CanShowZero` true _asnum_actor_2)
          (set `/Game/Blueprint/Mine/NumActor.CanShowZero` true _asnum_actor))))
    (:`then_1`
      (`/Game/Blueprint/Mine/NumActor.CreateNum` _asnum_actor_2 (mod _returnvalue 10))
      (`/Game/Blueprint/Mine/NumActor.CreateNum` _asnum_actor (/ _returnvalue 10)))))

(event `OpenDoor`
  (bind (_direction `_新建轨道_1`) (`Timeline|Open` :!via `PlayFromStart` :!label _label)
    (:`Update`
      (`SceneComponent.K2_SetRelativeLocation` (`self.StaticMesh1`) (+ (`KismetMathLibrary.MakeVector` (* (.x (`self.StaticMesh1Location`)) `_新建轨道_1`)) (`self.StaticMesh1Location`)) false false)
      (`SceneComponent.K2_SetRelativeLocation` (`self.StaticMesh2`) (+ (`KismetMathLibrary.MakeVector` (* `_新建轨道_1` (.x (`self.StaticMesh2Location`)))) (`self.StaticMesh2Location`)) false false))))

(event `CloseDoor`
  (goto _label :!via `ReverseFromEnd`))

(event `self.Box.OnComponentBeginOverlap`
  (params (OverlappedComponent :type "PrimitiveComponent Object Reference") (OtherActor :type "Actor Object Reference") (OtherComp :type "PrimitiveComponent Object Reference") (OtherBodyIndex :type Integer) (bFromSweep :type Boolean) (SweepResult :type "HitResult Structure (by ref)"))
  (cast `Character` OtherActor)
  (`self.LeaveDoor`))

(fn `UserConstructionScript`)