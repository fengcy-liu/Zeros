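; Cabinet actor with a hinged Cap component that swings open and closed through custom events.
; OpenCabinet and CloseCabinet each play their own timeline from the start, lerping the Cap's relative pitch between shut and open in opposite directions.
; BeginPlay caches the game mode and game instance, which are otherwise unused here.
; The AffactArea overlap events are empty, so nothing in this Blueprint triggers the lid.
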(event `self.ReceiveBeginPlay`
  (set `self.GameMode` (cast `/Game/Blueprint/Game/ATGameMode` (`GameplayStatics.GetGameMode`) :!pure true))
  (set `self.GameInstance` (cast `/Game/Blueprint/Game/ATGameInstance` (`GameplayStatics.GetGameInstance`) :!pure true)))

(event `self.AffactArea.OnComponentBeginOverlap`
  (params (OverlappedComponent :type "PrimitiveComponent Object Reference") (OtherActor :type "Actor Object Reference") (OtherComp :type "PrimitiveComponent Object Reference") (OtherBodyIndex :type Integer) (bFromSweep :type Boolean) (SweepResult :type "HitResult Structure (by ref)")))

(event `self.AffactArea.OnComponentEndOverlap`
  (params (OverlappedComponent :type "PrimitiveComponent Object Reference") (OtherActor :type "Actor Object Reference") (OtherComp :type "PrimitiveComponent Object Reference") (OtherBodyIndex :type Integer)))

(event `OpenCabinet`
  (bind (_direction _ratio) (`Timeline|时间轴_1` :!via `PlayFromStart`)
    (:`Update`
      (`SceneComponent.K2_SetRelativeRotation` (`self.Cap`) (`KismetMathLibrary.MakeRotator` 0.0 (`KismetMathLibrary.Lerp` 0.0 135.0 _ratio)) false false))))

(event `CloseCabinet`
  (bind (_direction _ratio) (`Timeline|时间轴_2` :!via `PlayFromStart`)
    (:`Update`
      (`SceneComponent.K2_SetRelativeRotation` (`self.Cap`) (`KismetMathLibrary.MakeRotator` 0.0 (`KismetMathLibrary.Lerp` 135.0 0.0 _ratio)) false false))))

(fn `UserConstructionScript`)