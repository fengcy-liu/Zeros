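; GlobalTimer drives the day/night cycle, converting game time into day, hour and minute, offset by a quarter day.
; Tick passes through a gate, which StopTimer closes, to update the clock and flip IsDayTime at hours 6 and 18, calling empty EnterDayTime/EnterNightTime events.
; Each update also sets sun pitch from the day fraction, refreshes the sky sphere and recaptures the skylight.
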(event `self.ReceiveBeginPlay`
  (bind (_returnvalue_roll _returnvalue_pitch) (`KismetMathLibrary.BreakRotator` (`self.K2_GetActorRotation` (`self.SunLight`))))
  (set `self.SunLightInitPitchValue` _returnvalue_pitch)
  (set `self.TimeOffset` (/ (`self.secondsPerDay`) 4.0)))

(event `StopTimer`
  (bind _secondsperday (`self.secondsPerDay`))
  (bind _currenthour (`self.CurrentHour`))
  (bind _isdaytime (`self.IsDayTime`))
  (bind _returnvalue (/ _secondsperday 24.0))
  (bind (_remainder _returnvalue_2) (`KismetMathLibrary.FMod` (+ (`KismetSystemLibrary.GetGameTimeInSeconds`) (`self.TimeOffset`)) _secondsperday))
  (bind (_remainder_2 _returnvalue_3) (`KismetMathLibrary.FMod` _remainder _returnvalue))
  (goto _label :!via `Close`))

(event `self.ReceiveTick`
  (params (DeltaSeconds :type "Float (single-precision)"))
  (bind _secondsperday (`self.secondsPerDay`))
  (bind _currenthour (`self.CurrentHour`))
  (bind _isdaytime (`self.IsDayTime`))
  (bind _returnvalue (/ _secondsperday 24.0))
  (bind (_remainder _returnvalue_2) (`KismetMathLibrary.FMod` (+ (`KismetSystemLibrary.GetGameTimeInSeconds`) (`self.TimeOffset`)) _secondsperday))
  (bind (_remainder_2 _returnvalue_3) (`KismetMathLibrary.FMod` _remainder _returnvalue))
  (`/Engine/EditorBlueprintResources/StandardMacros.Gate` false :!label _label
    (:`Exit`
      (`|ExecutionSequence`
        (:`then_0`
          (set `self.CurrentDay` _returnvalue_2)
          (set `self.CurrentHour` _returnvalue_3)
          (set `self.CurrentMinute` (`.ReturnValue` (`KismetMathLibrary.FMod` _remainder_2 (/ _returnvalue 60.0))))
          (if (xor _isdaytime (and (< _currenthour 18) (>= _currenthour 6)))
            (bind _output_get (set `self.IsDayTime` (not _isdaytime)))
            (if _output_get
              (`self.EnterDayTime`)
              (else
                (`self.EnterNightTime`)))))
        (:`then_1`
          (`self.K2_SetActorRotation` (`self.SunLight`) (`KismetMathLibrary.MakeRotator` 0.0 (+ (* (`KismetMathLibrary.Fraction` (/ (+ (`KismetSystemLibrary.GetGameTimeInSeconds`) (`self.TimeOffset`)) (`self.secondsPerDay`))) -360.0) 90.0)) false)
          (`/Engine/EngineSky/BP_Sky_Sphere.UpdateSunDirection` (`self.SkySphere`))
          (`SkyLightComponent.RecaptureSky` (`SkyLight.LightComponent` (`self.SkyLight`))))))))

(event `EnterDayTime`)

(event `EnterNightTime`)

(fn `UserConstructionScript`)