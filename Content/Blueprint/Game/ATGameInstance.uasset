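; Game instance that manages the game's UI panels (load screen, main menu, runtime HUD, pause and game over), button sounds and new-game start.
; ShowPanel lazily creates and caches each widget by reference, while HidePanel removes it, both optionally updating an open-panel counter.
; Game-only input returns only when that counter is zero.
; StartNewGame stores difficulty and restarts through ATGameMode; HideAllPanel hides only the HUD, and PushNewMessage is empty.
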(event `ShowLoadUI`
  ;[1 1 1] 界面
  (`self.HideAllPanel`)
  (`self.ShowPanel` "/Game/UI/UMG_LoadMenuUI.UMG_LoadMenuUI_C" (`self.LoadPanel`) false))

(event `PlayClickSound`
  ;[1 1 1] 播放按钮的音效
  (`GameplayStatics.PlaySound2D` "/Game/Sound/ButtonClick1.ButtonClick1" 1.0 1.0 0.0 null null))

(event `PlayFloatingSound`
  ;[1 1 1] 播放按钮的音效
  (`GameplayStatics.PlaySound2D` "/Game/Sound/ButtonFloating.ButtonFloating" 1.0 1.0 0.0 null null))

(event `HideLoadUI`
  ;[1 1 1] 界面
  (`self.HidePanel` (`self.LoadPanel`) false))

(event `ShowMainMenuUI`
  ;[1 1 1] 界面
  (`self.ShowPanel` "/Game/UI/UMG_StartMenu.UMG_StartMenu_C" (`self.StartMenuUI`))
  (`self.SetInputModeUIWithCursor` true))

(event `ShowRunTimeUI`
  ;[1 1 1] 界面
  (`self.ShowPanel` "/Game/UI/UMG_PlayerRunTimeUI.UMG_PlayerRunTimeUI_C" (`self.RunTimeUI`) false))

(event `PushNewMessage`
  (params (MessageText :type String))
  ;[1 1 1] 游戏逻辑
)

(event `StartNewGame`
  (params (Difficulty :type "/Game/Blueprint/Game/EnumGameDifficulty Enum" :default "EnumGameDifficulty_MAX"))
  ;[1 1 1] 游戏逻辑
  (set `self.Difficulty` Difficulty)
  (`self.HidePanel` (`self.StartMenuUI`))
  (`self.SetIpnputModeGameWithCursor` false
    (:`then`
      (bind _asatgame_mode (cast `/Game/Blueprint/Game/ATGameMode` (`GameplayStatics.GetGameMode`)))
      (`/Game/Blueprint/Game/ATGameMode.RestartGame` _asatgame_mode))))

(event `ShowGameOverPanel`
  (params (Message :type String) (InColorAndOpacity :type "SlateColor Structure") (IsSuccess :type Boolean))
  ;[1 1 1] 界面
  (`self.HideAllPanel`)
  (`self.ShowPanel` "/Game/UI/UMG_GameOver.UMG_GameOver_C" (`self.GameOverUI`))
  (`self.SetInputModeUIWithCursor` true)
  (`/Game/UI/UMG_GameOver.SetGameOverMessage` (`self.GameOverUI`) Message InColorAndOpacity IsSuccess))

(event `ShowPausePanel`
  ;[1 1 1] 界面
  (`self.ShowPanel` "/Game/UI/UMG_PauseMenu.UMG_PauseMenu_C" (`self.PausePanel`))
  (`self.SetInputModeUIWithCursor` true))

(event `HidePausePanel`
  ;[1 1 1] 界面
  (`self.HidePanel` (`self.PausePanel`))
  (`self.SetIpnputModeGameWithCursor` false
    (:`then`
      (`self.ShowPanel` "/Game/UI/UMG_PlayerRunTimeUI.UMG_PlayerRunTimeUI_C" (`self.RunTimeUI`)))))

(event `HideAllPanel`
  ;[1 1 1] 界面
  (`|ExecutionSequence`
    (:`then_0`
      (`self.HidePanel` (`self.RunTimeUI`) false))))

(fn `HidePanel`
  (params (TargetPanel :type "Widget Object Reference") (bChangeInputMode :type Boolean :default true))
  (`/Engine/EditorBlueprintResources/StandardMacros.IsValid` TargetPanel
    (:`Is Valid`
      (if (`Widget.IsVisible` TargetPanel)
        (`Widget.RemoveFromParent` TargetPanel)
        (if bChangeInputMode
          (`/Engine/EditorBlueprintResources/StandardMacros.DecrementInt` (`self.ActiveUICount`)
            (:`  `
              (return)))
          (else
            (return)))))))

(fn `IsAllPanelClosed`
  (returns (ReturnValue :type Boolean))
  (return (== (`self.ActiveUICount`) 0)))

(fn `ShowPanel`
  (params (PanelTypeClass :type "UserWidget Class Reference") (TargetPanel :type "UserWidget Object Reference (by ref)") (bChangeInputMode :type Boolean :default true))
  (`/Engine/EditorBlueprintResources/StandardMacros.IsValid` TargetPanel
    (:`Is Valid`
      (if (not (`Widget.IsInViewport` TargetPanel))
        (`UserWidget.AddToViewport` TargetPanel 0 :!label _label)
        (if bChangeInputMode
          (`/Engine/EditorBlueprintResources/StandardMacros.IncrementInt` (`self.ActiveUICount`)
            (:`  `
              (return)))
          (else
            _))))
    (:`Is Not Valid`
      (bind _returnvalue (`|CreateWidget` PanelTypeClass (`GameplayStatics.GetPlayerController` 0)))
      (`|VariableSetRef` TargetPanel _returnvalue)
      (goto _label)))
  (return))