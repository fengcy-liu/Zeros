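; ATGameMode controls session flow: loading, pause and resume, game over, restart and exit.
; Panels are shown and hidden through ATGameInstance, whose IsPlayerRunTime flag makes BeginPlay start the loading sequence, as after a restart reopens MineMap.
; Loading progress is simulated: a Tick-driven, re-armed DoOnce advances LoadPercent over about three seconds, then after a short delay switches to game-only input and runtime UI.
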(event `self.ReceiveBeginPlay`
  (set `self.GameInstance` (cast `/Game/Blueprint/Game/ATGameInstance` (`GameplayStatics.GetGameInstance`) :!pure true))
  (set `/Game/Blueprint/Game/ATGameInstance.ActiveUICount` 0 (`self.GameInstance`))
  (if (`/Game/Blueprint/Game/ATGameInstance.IsPlayerRunTime` (`self.GameInstance`))
    (`/Game/Blueprint/Game/ATGameInstance.ShowLoadUI` (`self.GameInstance`))
    (`self.LoadProcess_false`)))

(event `GameOver`
  (params (Message :type String) (InColorAndOpacity :type "SlateColor Structure") (IsSuccess :type Boolean))
  (set `/Game/Blueprint/Game/ATGameInstance.IsPlayerRunTime` false (`self.GameInstance`))
  (`/Game/Blueprint/Game/ATGameInstance.ShowGameOverPanel` (`self.GameInstance`) Message InColorAndOpacity IsSuccess))

(event `RestartGame`
  (set `/Game/Blueprint/Game/ATGameInstance.IsPlayerRunTime` true (`self.GameInstance`))
  (`GameplayStatics.OpenLevelBySoftObjectPtr` "/Game/Maps/MineMap.MineMap"))

(event `ExitGame`
  (`KismetSystemLibrary.ExecuteConsoleCommand` "exit" null))

(event `LoadProcess_false`
  (bind _gameinstance (`self.GameInstance`))
  (goto _label :!via `Reset`))

(event `self.ReceiveTick`
  (params (DeltaSeconds :type "Float (single-precision)"))
  (bind _gameinstance (`self.GameInstance`))
  (`/Engine/EditorBlueprintResources/StandardMacros.DoOnce` true :!label _label
    (:`Completed`
      (bind _output_get (set `self.LoadPercent` (`KismetMathLibrary.FClamp` (+ (`self.LoadPercent`) (/ (`GameplayStatics.GetWorldDeltaSeconds`) 3.0)))))
      (if (>= _output_get 1.0)
        (`KismetSystemLibrary.Delay` 1.0)
        (`WidgetBlueprintLibrary.SetInputMode_GameOnly` (`GameplayStatics.GetPlayerController` 0))
        (`/Game/Blueprint/Game/ATGameInstance.HideLoadUI` _gameinstance)
        (`/Game/Blueprint/Game/ATGameInstance.ShowRunTimeUI` _gameinstance)
        (else
          (goto _label :!via `Reset`))))))

(event `PauseGame`
  (`GameplayStatics.SetGamePaused` true)
  (`/Game/Blueprint/Game/ATGameInstance.ShowPausePanel` (`self.GameInstance`)))

(event `ResumeGame`
  (`GameplayStatics.SetGamePaused` false)
  (`/Game/Blueprint/Game/ATGameInstance.HidePausePanel` (`self.GameInstance`)))

(fn `UserConstructionScript`)